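; Flyer actor that carries its cylinder from a start point to an end point when the player triggers it.
; A box trigger enables the player's input on the actor while the third-person character overlaps it, and disables it on exit.
; Pressing G plays the MoveFlyer timeline, which lerps the cylinder's relative location between StartPoint and EndPoint without sweeping.
; Only forward playback is wired, with no return movement.
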(event OnComponentBeginOverlap(Box)
  (params (OverlappedComponent :type Primitive%20Component%20Object%20Reference) (OtherActor :type Actor%20Object%20Reference) (OtherComp :type Primitive%20Component%20Object%20Reference) (OtherBodyIndex :type Integer) (bFromSweep :type Boolean) (SweepResult :type Hit%20Result%20Structure%20%28by%20ref%29))
  (Utilities|Casting|CastToThirdPersonCharacter OtherActor)
  (Input|EnableInput (Game|GetPlayerController 0)))

(event OnComponentEndOverlap(Box)
  (params (OverlappedComponent :type Primitive%20Component%20Object%20Reference) (OtherActor :type Actor%20Object%20Reference) (OtherComp :type Primitive%20Component%20Object%20Reference) (OtherBodyIndex :type Integer))
  (Utilities|Casting|CastToThirdPersonCharacter OtherActor)
  (Input|DisableInput (Game|GetPlayerController 0)))

(event Input|KeyboardEvents|G
  (params (Key :type Key%20Structure :default "None"))
  (:Pressed
    (bind _move_flyer (Timeline|Move%20Flyer Play)
      (:Update
        (Transformation|SetRelativeLocation (Variables|Default|GetFlyer_Cylinder) (Math|Vector|Lerp(Vector) (Variables|Default|GetStartPoint) (Variables|Default|GetEndPoint) _move_flyer) false false)))))

(fn ConstructionScript)